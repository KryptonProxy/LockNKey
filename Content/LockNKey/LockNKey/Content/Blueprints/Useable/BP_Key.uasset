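; BP_Key is a key pickup that the player collects by pressing E while something overlaps its box.
; Box overlap enables player input on the actor and opens a Gate, and ending the overlap reverses both.
; A gated E press calls AddKey on the overlapping actor, plays the pickup cue at the key's location through a PlaySound helper, and destroys the key.
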(event OnComponentBeginOverlap(Box)
  (params (OverlappedComponent :type Primitive%20Component%20Object%20Reference) (OtherActor :type Actor%20Object%20Reference) (OtherComp :type Primitive%20Component%20Object%20Reference) (OtherBodyIndex :type Integer) (bFromSweep :type Boolean) (SweepResult :type Hit%20Result%20Structure%20%28by%20ref%29))
  ;[1 1 1] Interact w/ Key
  (Input|EnableInput (Game|GetPlayerController 0))
  (Utilities|FlowControl|Gate true) ; enters at Open
)

(event OnComponentEndOverlap(Box)
  (params (OverlappedComponent :type Primitive%20Component%20Object%20Reference) (OtherActor :type Actor%20Object%20Reference) (OtherComp :type Primitive%20Component%20Object%20Reference) (OtherBodyIndex :type Integer))
  ;[1 1 1] Interact w/ Key
  (Input|DisableInput (Game|GetPlayerController 0))
  (Utilities|FlowControl|Gate true) ; enters at Close
)

(event EventBeginPlay)

(event Collision|EventActorBeginOverlap
  (params (OtherActor :type Actor%20Object%20Reference)))

(event EventTick
  (params (DeltaSeconds :type Float%20%28single-precision%29)))

(event Input|KeyboardEvents|E
  (params (Key :type Key%20Structure :default "None"))
  ;[1 1 1] Interact w/ Key
  (:Pressed
    (Utilities|FlowControl|Gate true
      (:Exit
        (AddComponent|AddKey (stale OnComponentBeginOverlap(Box) OtherActor))
        (Utilities|PlaySound "/LockNKey/Sounds/Cues/keypickup_Cue.keypickup_Cue")
        (Actor|DestroyActor)))))

(fn ConstructionScript)