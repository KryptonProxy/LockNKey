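; BP_LockedDoor is a door that the player can open and close with E once an actor carrying a Key component overlaps its Box.
; That overlap enables input and opens a gate; a keyless overlap calls a sound macro, disables input and closes the gate, with no end-overlap handling.
; E passes through the gate to a FlipFlop that plays or reverses a timeline, lerping DoorMesh yaw between closed and open angles.
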(event OnComponentBeginOverlap(Box)
  (params (OverlappedComponent :type Primitive%20Component%20Object%20Reference) (OtherActor :type Actor%20Object%20Reference) (OtherComp :type Primitive%20Component%20Object%20Reference) (OtherBodyIndex :type Integer) (bFromSweep :type Boolean) (SweepResult :type Hit%20Result%20Structure%20%28by%20ref%29))
  (bind _returnvalue (Game|GetPlayerController 0))
  ;[1 1 1] Open Door w/ Key
  (Utilities|IsValid (Actor|GetComponentbyClass OtherActor "/Game/01_Blueprints/Key.Key_C")
    (:Is%20Valid
      (Input|EnableInput _returnvalue)
      (Utilities|FlowControl|Gate true) ; enters at Open
    )
    (:Is%20Not%20Valid
      (Utilities|NewMacro0)
      (Input|DisableInput _returnvalue)
      (Utilities|FlowControl|Gate true) ; enters at Close
    )))

(event EventBeginPlay)

(event Collision|EventActorBeginOverlap
  (params (OtherActor :type Actor%20Object%20Reference)))

(event EventTick
  (params (DeltaSeconds :type Float%20%28single-precision%29)))

(event Input|KeyboardEvents|E
  (params (Key :type Key%20Structure :default "None"))
  ;[1 1 1] Open Door w/ Key
  (:Pressed
    (Utilities|FlowControl|Gate true
      (:Exit
        ;[1 1 1] Door Anim
        (Utilities|FlowControl|FlipFlop
          (:A
            (bind _door (Timeline|Open/Close%20Door Play)
              (:Update
                (Transformation|SetRelativeRotation (Variables|Default|GetDoorMesh) (Math|Rotator|MakeRotator 0.0 0.0 (Math|Float|Lerp (Variables|Default|GetClosedAngle) (Variables|Default|GetOpenAngle) _door)) false false))))
          (:B
            (Timeline|Open/Close%20Door Reverse)))))))

(fn ConstructionScript)